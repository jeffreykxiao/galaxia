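; EnemyProjectile is a projectile Blueprint that damages Friendly-tagged actors it overlaps.
; On overlap it handles only actors implementing the IDamagable interface, then branches on their actor tags.
; An Enemy tag triggers an IgnoreActorWhenMoving call on ProjectileCollision, with no actor specified.
; A Friendly tag sends Damage through the AffectHealthMessage interface call and destroys the projectile.
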(event EventBeginPlay)

(event Collision|EventActorBeginOverlap
  (params (OtherActor :type Actor%20Object%20Reference))
  (if (Utilities|DoesObjectImplementInterface OtherActor "/Game/Blueprints/iDamagable.iDamagable_C")
    (if (Actor|ActorHasTag OtherActor "Enemy")
      (Collision|IgnoreActorwhenMoving (Variables|Default|GetProjectileCollision) 0 true)
      (elif (Actor|ActorHasTag OtherActor "Friendly")
        (Class|IDamagable|AffectHealth(Message) OtherActor (Variables|Default|GetDamage))
        (Actor|DestroyActor)))))

(event EventTick
  (params (DeltaSeconds :type Float%20%28single-precision%29)))

(fn ConstructionScript)