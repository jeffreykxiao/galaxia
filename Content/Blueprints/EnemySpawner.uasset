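; EnemySpawner is an actor that spawns AI enemies of two types, Enemy2 and Enemy3, at random points inside its SpawnVolume box.
; Separate SpawnEnemy2 and SpawnEnemy3 events count live actors of their class in the level and spawn one only while below that type's max limit.
; The Blueprint does not trigger these events itself, as BeginPlay, Tick and overlap are unused.
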(event Custom|SpawnEnemy2
  (bind _spawn_volume (Variables|Default|GetSpawn%20Volume))
  (bind _outactors (Actor|GetAllActorsOfClass "/Game/Blueprints/Enemy2.Enemy2_C"))
  (if (< (Utilities|Array|Length _outactors) (Variables|Default|GetMaxEnemies2))
    (AI|SpawnAIFromClass "/Game/Blueprints/Enemy2.Enemy2_C" 0 (Math|Random|RandomPointinBoundingBox (Transformation|GetWorldLocation _spawn_volume) (Components|Box|GetScaledBoxExtent _spawn_volume)) "0, 0, 0" false)))

(event Custom|SpawnEnemy3
  (bind _spawn_volume (Variables|Default|GetSpawn%20Volume))
  (bind _outactors (Actor|GetAllActorsOfClass "/Game/Blueprints/Enemy3.Enemy3_C"))
  (if (< (Utilities|Array|Length _outactors) (Variables|Default|GetMaxEnemies3))
    (AI|SpawnAIFromClass "/Game/Blueprints/Enemy3.Enemy3_C" 0 (Math|Random|RandomPointinBoundingBox (Transformation|GetWorldLocation _spawn_volume) (Components|Box|GetScaledBoxExtent _spawn_volume)) "0, 0, 0" false)))

(event EventBeginPlay)

(event Collision|EventActorBeginOverlap
  (params (OtherActor :type Actor%20Object%20Reference)))

(event EventTick
  (params (DeltaSeconds :type Float%20%28single-precision%29)))

(fn ConstructionScript)