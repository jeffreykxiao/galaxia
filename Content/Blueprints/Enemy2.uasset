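; Twin-stick shooter enemy that damages the hero on contact and is drawn with eight-direction flipbook sprites.
; Hero overlap starts a looping damage timer, which end overlap tries to clear by function name.
; AffectHealth handles death by adding score, destroying the actor and randomly spawning a scaled-down Powerup.
; Tick maps actor yaw to a facing state and velocity to idle or moving, then selects the matching flipbook.
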(event Custom|Damage%20Hero
  (Default|AffectHealth (Variables|Default|GetHero) (Variables|Default|GetDamage)))

(event EventBeginPlay)

(event Collision|EventActorBeginOverlap
  (params (OtherActor :type Actor%20Object%20Reference))
  (bind _ashero_character_2 (Utilities|Casting|CastToHeroCharacter2 OtherActor))
  (Variables|Default|SetHero _ashero_character_2)
  (Utilities|Time|SetTimerbyEvent (delegate Custom|Damage%20Hero) (/ 1.0 (Variables|Default|GetAttacks%20per%20sec)) true)
  (bind _aspowerup (Utilities|Casting|CastToPowerup OtherActor))
  (Variables|Default|SetPowerUp _aspowerup))

(event Collision|EventActorEndOverlap
  (params (OtherActor :type Actor%20Object%20Reference))
  (if (== OtherActor (Variables|Default|GetHero))
    (Utilities|Time|ClearTimerbyFunctionName 0 "Damage Hero")))

(event EventTick
  (params (DeltaSeconds :type Float%20%28single-precision%29))
  (Variables|Default|Setis%20Idle (== (Math|Vector|VectorLength (Transformation|GetVelocity)) 0.0))
  (Variables|Default|SetIs%20Moving (> (Math|Vector|VectorLength (Transformation|GetVelocity)) 0.0))
  ;[1 1 1] Rotation States
  (Variables|Default|SetIs%20Facing%20Front (Math|Float|NearlyEqual(Float) (.Yaw (Math|Rotator|BreakRotator (Transformation|GetActorRotation))) 1.8e+02 1e+01))
  (Variables|Default|SetIs%20Facing%20Back (Math|Float|NearlyEqual(Float) (.Yaw (Math|Rotator|BreakRotator (Transformation|GetActorRotation))) 0.0 22.5))
  (Variables|Default|SetIs%20Facing%20Left (Math|Float|NearlyEqual(Float) (.Yaw (Math|Rotator|BreakRotator (Transformation|GetActorRotation))) 9e+01 22.5))
  (Variables|Default|SetIs%20Facing%20Right (Math|Float|NearlyEqual(Float) (.Yaw (Math|Rotator|BreakRotator (Transformation|GetActorRotation))) -9e+01 22.5))
  (Variables|Default|SetIs%20Facing%20Back%20Left (Math|Float|NearlyEqual(Float) (.Yaw (Math|Rotator|BreakRotator (Transformation|GetActorRotation))) 45.0 22.5))
  (Variables|Default|SetIs%20Facing%20Back%20Right (Math|Float|NearlyEqual(Float) (.Yaw (Math|Rotator|BreakRotator (Transformation|GetActorRotation))) -45.0 22.5))
  (Variables|Default|SetIs%20Facing%20Front%20Right (Math|Float|NearlyEqual(Float) (.Yaw (Math|Rotator|BreakRotator (Transformation|GetActorRotation))) -135.0 22.5))
  (Variables|Default|SetIs%20Facing%20Front%20Left (Math|Float|NearlyEqual(Float) (.Yaw (Math|Rotator|BreakRotator (Transformation|GetActorRotation))) 135.0 22.5))
  (if (Variables|Default|GetIs%20Facing%20Front)
    (Variables|Default|SetFacing%20State "NewEnumerator0")
    (if (Variables|Default|GetIs%20Moving) :!label _label
      (Sprite|SetFlipbook (Variables|Default|GetPaperFlipbook) (Utilities|Select :Index (Variables|Default|GetFacing%20State) :NewEnumerator0 "/Game/AnimationAssets/GalaxiaTempAssets/Moving/Front/Moving_Front.Moving_Front" :NewEnumerator1 "/Game/AnimationAssets/GalaxiaTempAssets/Moving/Back/Moving_Back.Moving_Back" :NewEnumerator2 "/Game/AnimationAssets/GalaxiaTempAssets/Moving/FrontLeft/Moving_FrontLeft.Moving_FrontLeft" :NewEnumerator3 "/Game/AnimationAssets/GalaxiaTempAssets/Moving/Left/Moving_Left.Moving_Left" :NewEnumerator4 "/Game/AnimationAssets/GalaxiaTempAssets/Moving/BackLeft/Moving_BackLeft.Moving_BackLeft" :NewEnumerator5 "/Game/AnimationAssets/GalaxiaTempAssets/Moving/BackRight/Moving_BackRight.Moving_BackRight" :NewEnumerator6 "/Game/AnimationAssets/GalaxiaTempAssets/Moving/Right/Moving_Right.Moving_Right" :NewEnumerator7 "/Game/AnimationAssets/GalaxiaTempAssets/Moving/FrontRight/Moving_FrontRight.Moving_FrontRight"))
      (elif (Variables|Default|Getis%20Idle)
        (Sprite|SetFlipbook (Variables|Default|GetPaperFlipbook) (Utilities|Select :Index (Variables|Default|GetFacing%20State) :NewEnumerator0 "/Game/AnimationAssets/GalaxiaTempAssets/Idle/Front/Idle_Front.Idle_Front" :NewEnumerator1 "/Game/AnimationAssets/GalaxiaTempAssets/Idle/Back/Idle_Back.Idle_Back" :NewEnumerator2 "/Game/AnimationAssets/GalaxiaTempAssets/Idle/FrontLeft/Idle_FrontLeft.Idle_FrontLeft" :NewEnumerator3 "/Game/AnimationAssets/GalaxiaTempAssets/Idle/Left/Idle_Left.Idle_Left" :NewEnumerator4 "/Game/AnimationAssets/GalaxiaTempAssets/Idle/BackLeft/Idle_BackLeft.Idle_BackLeft" :NewEnumerator5 "/Game/AnimationAssets/GalaxiaTempAssets/Idle/BackRight/Idle_BackRight.Idle_BackRight" :NewEnumerator6 "/Game/AnimationAssets/GalaxiaTempAssets/Idle/Right/Idle_Right.Idle_Right" :NewEnumerator7 "/Game/AnimationAssets/GalaxiaTempAssets/Idle/FrontRight/Idle_FrontRight.Idle_FrontRight"))))
    (elif (Variables|Default|GetIs%20Facing%20Back)
      (Variables|Default|SetFacing%20State "NewEnumerator1")
      (goto _label)
      (elif (Variables|Default|GetIs%20Facing%20Left)
        (Variables|Default|SetFacing%20State "NewEnumerator3")
        (goto _label)
        (elif (Variables|Default|GetIs%20Facing%20Right)
          (Variables|Default|SetFacing%20State "NewEnumerator6")
          (goto _label)
          (elif (Variables|Default|GetIs%20Facing%20Front%20Right)
            (Variables|Default|SetFacing%20State "NewEnumerator7")
            (goto _label)
            (elif (Variables|Default|GetIs%20Facing%20Front%20Left)
              (Variables|Default|SetFacing%20State "NewEnumerator2")
              (goto _label)
              (elif (Variables|Default|GetIs%20Facing%20Back%20Left)
                (Variables|Default|SetFacing%20State "NewEnumerator4")
                (goto _label)
                (elif (Variables|Default|GetIs%20Facing%20Back%20Right)
                  (Variables|Default|SetFacing%20State "NewEnumerator5")
                  (goto _label))))))))))

(event EventAffectHealth
  (params (Delta :type Float%20%28single-precision%29))
  (bind _returnvalue (Transformation|GetActorTransform))
  (bind (_location _rotation) (Math|Transform|BreakTransform _returnvalue))
  (Class|MyCharacter|CalculateHealth Delta)
  (if (Variables|Default|GetisDead)
    (bind _astwin_stick_mode (Utilities|Casting|CastToTwinStickMode (Game|GetGameMode)))
    (Default|IncrementScore _astwin_stick_mode 300)
    (Actor|DestroyActor)
    (if (<= (Math|Random|RandomFloat) (Variables|Default|GetPowerUp%20Spawn%20Chance))
      (Game|SpawnActorfromClass "/Game/Blueprints/Powerup.Powerup_C" (Math|Transform|MakeTransform _location _rotation "0.300000,0.300000,0.300000") "Undefined" 0 0))))

(fn ConstructionScript)